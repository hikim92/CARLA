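; Audi TT CARLA vehicle for Viaduct, with an in-car HMI that shows driver-assistance state when it is the hero car.
; Each Tick copies ViaductPlayerController HUD values into ACC and speed-limit readouts, warning icons, mirror alerts and turn indicators.
; Nested FlipFlops throttle the absolute forward-speed text to every eighth tick.
; SetUserPawn stops the three mirror components ticking on non-hero cars.
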(event EventBeginPlay
  (|CallParentFunction))

(event Collision|EventActorBeginOverlap
  (params (OtherActor :type Actor%20Object%20Reference)))

(event EventTick
  (params (DeltaSeconds :type Float%20%28single-precision%29))
  (bind _viaductplayercontroller (Variables|Default|GetViaductPlayerController))
  (bind _hmi_speed_acc (Variables|Default|GetHMI_Speed_ACC))
  (bind _viaductplayercontroller_2 (Variables|Default|GetViaductPlayerController))
  (bind _hud_speed_limit (Variables|/Script/CarlaUE4.ViaductPlayerController|GetHUD_SPEED_LIMIT _viaductplayercontroller_2))
  (|CallParentFunction DeltaSeconds)
  (if (Variables|Default|GetIsHero)
    (Utilities|FlowControl|Sequence
      (:then_0
        ;[0.8016 1 0.7659] HMI Speed
        (Utilities|FlowControl|FlipFlop
          (:B
            (Utilities|FlowControl|FlipFlop
              (:B
                (Utilities|FlowControl|FlipFlop
                  (:B
                    (Rendering|Components|TextRender|SetText (Variables|Default|GetHMI_Speed) (Utilities|Text|ToText(Float) (Math|Float|Absolute(Float) (Class|CarlaWheeledVehicle|GetVehicleForwardSpeed)) "HalfToEven" false true 1 999 0 0)))))))))
      (:then_1
        ;[1 0.966 0.581] ACC & Speed Limit
        (Utilities|FlowControl|Sequence
          (:then_0
            (Rendering|Components|TextRender|SetText _hmi_speed_acc (Utilities|Text|ToText(Integer) (Variables|/Script/CarlaUE4.ViaductPlayerController|GetHUD_ACC_SPEED _viaductplayercontroller_2)))
            (Rendering|SetVisibility _hmi_speed_acc (Variables|/Script/CarlaUE4.ViaductPlayerController|GetHUD_ACC _viaductplayercontroller_2) true))
          (:then_1
            (Rendering|Components|TextRender|SetText (Variables|Default|GetHMI_Speed_Limit) (Utilities|Text|ToText(Integer) _hud_speed_limit))
            (Rendering|SetVisibility (Variables|Default|GetHMI_Speed_Limit_bg) (>= _hud_speed_limit 10) true))))
      (:then_2
        ;[1 0.4991 0.4092] Warning
        (Utilities|FlowControl|Sequence
          (:then_0
            (Rendering|SetVisibility (Variables|Default|GetHMI_FCW) (Variables|/Script/CarlaUE4.ViaductPlayerController|GetHUD_FCW _viaductplayercontroller) false))
          (:then_1
            (Rendering|SetVisibility (Variables|Default|GetHMI_AEB) (Variables|/Script/CarlaUE4.ViaductPlayerController|GetHUD_AEB _viaductplayercontroller) false))
          (:then_2
            (Rendering|SetVisibility (Variables|Default|GetHMI_LDW) (Variables|/Script/CarlaUE4.ViaductPlayerController|GetHUD_LDW _viaductplayercontroller) false))
          (:then_3
            (Rendering|SetVisibility (Variables|Default|GetMirror_Left_Warning_0) (Variables|/Script/CarlaUE4.ViaductPlayerController|GetHUD_MIRROR_W_LEFT _viaductplayercontroller) false))
          (:then_4
            (Rendering|SetVisibility (Variables|Default|GetMirror_Right_Warning) (Variables|/Script/CarlaUE4.ViaductPlayerController|GetHUD_MIRROR_W_RIGHT _viaductplayercontroller) false))
          (:then_5
            (Rendering|SetVisibility (Variables|Default|GetHMI_Turn_Left) (Variables|/Script/CarlaUE4.ViaductPlayerController|GetHUD_TURN_LEFT _viaductplayercontroller) false))
          (:then_6
            (Rendering|SetVisibility (Variables|Default|GetHMI_Turn_Right) (Variables|/Script/CarlaUE4.ViaductPlayerController|GetHUD_TURN_RIGHT _viaductplayercontroller) false))
          (:then_7
            (Rendering|SetVisibility (Variables|Default|GetHMI_LKA) (Variables|/Script/CarlaUE4.ViaductPlayerController|GetHUD_LKA _viaductplayercontroller) false))
          (:then_8
            (Rendering|SetVisibility (Variables|Default|GetHMI_LKA_OFF) (Variables|/Script/CarlaUE4.ViaductPlayerController|GetHUD_LKA_DISABLE _viaductplayercontroller) false))
          (:then_9
            (Rendering|SetVisibility (Variables|Default|GetHMI_ACC) (Variables|/Script/CarlaUE4.ViaductPlayerController|GetHUD_ACC _viaductplayercontroller) false))
          (:then_10
            (Rendering|SetVisibility (Variables|Default|GetHMI_ACC_OFF) (Variables|/Script/CarlaUE4.ViaductPlayerController|GetHUD_ACC_DISABLE _viaductplayercontroller) false))
          (:then_11
            (Rendering|SetVisibility (Variables|Default|GetHMI_Blinker_Left) (Variables|/Script/CarlaUE4.ViaductPlayerController|GetHUD_BLINKER_LEFT _viaductplayercontroller) false))
          (:then_12
            (Rendering|SetVisibility (Variables|Default|GetHMI_Blinker_Right) (Variables|/Script/CarlaUE4.ViaductPlayerController|GetHUD_BLINKER_RIGHT _viaductplayercontroller) false)))))))

(fn ConstructionScript
  (|CallParentFunction))

(fn SetUserPawn
  (params (isHero :type Boolean))
  (|CallParentFunction isHero)
  (if (not isHero)
    (Utilities|FlowControl|Sequence
      (:then_0
        (Components|Tick|SetComponentTickEnabled (Variables|Default|GetMirror_Left) false)))))